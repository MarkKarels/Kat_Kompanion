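; Collectable paw pickup that adds a paw point to the game instance when the Protagonist touches it.
; A looping-style bob and spin of the Paw is driven by the Float timeline from BeginPlay.
; The first overlap records the pickup in the level save object, plays sound and Niagara effects, then runs a scale timeline.
; When that timeline finishes, the actor is destroyed and PawPoints increments.
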(event `self.ReceiveBeginPlay`
  ;[0.1812 0 1] Float Animation
  (bind (_direction _height _rotation) (`Timeline|Float` :!via `PlayFromStart`)
    (:`Update`
      (`SceneComponent.K2_SetRelativeLocation` (`self.Paw`) (`KismetMathLibrary.MakeVector` 0.0 0.0 (`KismetMathLibrary.Lerp` 0.0 20.0 _height)) false false)
      (`SceneComponent.K2_SetWorldRotation` (`self.Paw`) (`KismetMathLibrary.MakeRotator` 0.0 0.0 (`KismetMathLibrary.Lerp` 0.0 360.0 _rotation)) false false))))

(event `self.Sphere.OnComponentBeginOverlap`
  (params (OverlappedComponent :type "PrimitiveComponent Object Reference") (OtherActor :type "Actor Object Reference") (OtherComp :type "PrimitiveComponent Object Reference") (OtherBodyIndex :type Integer) (bFromSweep :type Boolean) (SweepResult :type "HitResult Structure (by ref)"))
  ;[0.1812 0 1] Pickup
  (bind _asprotagonist (cast `/Game/ThirdPerson/Blueprints/Protagonist` OtherActor))
  (`/Engine/EditorBlueprintResources/StandardMacros.DoOnce` false
    (:`Completed`
      (`KismetArrayLibrary.Array_AddUnique` (`/Game/ThirdPerson/Blueprints/LevelDataObject.CollectedPickups` (`/Game/GameModes/Main_Play.LevelSaveObject` (`/Game/ThirdPerson/Blueprints/Protagonist.GameMode` _asprotagonist))) self)
      (`GameplayStatics.PlaySoundAtLocation` "/Game/Audio/Cue/PawPickup3.PawPickup3" (`SceneComponent.K2_GetComponentLocation` (`self.DefaultSceneRoot`)) (struct) 1.0 1.0 0.0 null null null null)
      (`NiagaraFunctionLibrary.SpawnSystemAtLocation` "/Game/EasyHealthSystem/Demo/Particles/NS_ShieldPotion.NS_ShieldPotion" (`self.K2_GetActorLocation`))
      (bind (_direction _scale) (`Timeline|DestroyAnimation` :!via `PlayFromStart`)
        (:`Update`
          (`SceneComponent.K2_SetRelativeTransform` (`self.Paw`) (`KismetMathLibrary.MakeTransform` (0.0 0.0 0.0) (struct) (`KismetMathLibrary.VLerp` (0.0 0.0 0.0) (0.5 0.5 0.5) _scale)) false false))
        (:`Finished`
          (`self.K2_DestroyActor`)
          (bind _asmy_game_instance (cast `/Game/Doors/MyGameInstance` (`GameplayStatics.GetGameInstance`)))
          (bind _result (`/Engine/EditorBlueprintResources/StandardMacros.IncrementInt` (`/Game/Doors/MyGameInstance.PawPoints` _asmy_game_instance))
            (:`  `
              (set `/Game/Doors/MyGameInstance.PawPoints` _result _asmy_game_instance))))))))

(fn `UserConstructionScript`)