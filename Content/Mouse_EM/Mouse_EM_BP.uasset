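; Mouse enemy pawn that chases the player's Kat_1_BP character and damages actors it touches.
; FollowPlayer, not triggered in this graph, checks a flag and re-runs after short delays, using AIMoveTo to approach the player or target itself when close; StopMovement enters that self-targeting branch.
; Sphere overlaps damage any actor with BPC_EasyHealthSystem.
; AnyDamage lowers its own Health, and Tick destroys it at zero.
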(event `self.ReceiveBeginPlay`
  (bind _askat_1_bp (cast `/Game/ThirdPerson/Blueprints/Kat_1_BP` (`GameplayStatics.GetPlayerCharacter` 0)))
  (set `self.Char REF` _askat_1_bp))

(event `Follow Player`
  (if (`self.FollowPlayer?`)
    (if (>= (`self.GetDistanceTo` (`self.Char REF`)) 200.0)
      (`|AIMoveTo` self (0.0 0.0 0.0) (`self.Char REF`)
        (:`then`
          _))
      (else
        (`|AIMoveTo` self (0.0 0.0 0.0) self :!label _label
          (:`then`
            _))))
    (`KismetSystemLibrary.Delay` 0.1)
    (`self.Follow Player`)))

(event `Stop Movement`
  (goto _label))

(event `self.Sphere.OnComponentBeginOverlap`
  (params (OverlappedComponent :type "PrimitiveComponent Object Reference") (OtherActor :type "Actor Object Reference") (OtherComp :type "PrimitiveComponent Object Reference") (OtherBodyIndex :type Integer) (bFromSweep :type Boolean) (SweepResult :type "HitResult Structure (by ref)"))
  (bind _returnvalue (`self.GetComponentByClass` OtherActor "/Game/EasyHealthSystem/Blueprints/BPC_EasyHealthSystem.BPC_EasyHealthSystem_C"))
  (`/Engine/EditorBlueprintResources/StandardMacros.IsValid` _returnvalue
    (:`Is Valid`
      (`/Game/EasyHealthSystem/Blueprints/BPC_EasyHealthSystem.TakeDamage` _returnvalue (`self.Damage`)))))

(event `self.ReceiveAnyDamage`
  (params (Damage :type "Float (single-precision)") (DamageType :type "DamageType Object Reference") (InstigatedBy :type "Controller Object Reference") (DamageCauser :type "Actor Object Reference"))
  (bind _health (`self.Health`))
  (if (> _health 0.0)
    (set `self.Health` (- _health Damage))
    (`KismetSystemLibrary.PrintString` "DMG")))

(event `self.ReceiveTick`
  (params (DeltaSeconds :type "Float (single-precision)"))
  (if (<= (`self.Health`) 0.0)
    (`self.K2_DestroyActor`)))

(fn `UserConstructionScript`)