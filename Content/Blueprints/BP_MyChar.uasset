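; BP_MyChar is a character Blueprint that demonstrates opening and responding to a radial menu.
; Pressing B creates a BP_Radialmenu widget, adds it to the viewport, registers itself as the menu's interface and shows the mouse cursor.
; The interface callbacks play an explosion sound on hover, and on click remove the menu and play a different explosion sound.
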(event `Key|B`
  (params (Key :type "Key Structure"))
  ;[1 1 1] Open Menu
  (:`Pressed`
    (bind _returnvalue (`|CreateWidget` "/Game/Blueprints/UI/BP_Radialmenu.BP_Radialmenu_C"))
    (`UserWidget.AddToViewport` _returnvalue 0)
    (`DzX_RadialMenu.SetRadMenuInterface` _returnvalue self)
    (set `PlayerController.bShowMouseCursor` true (`GameplayStatics.GetPlayerController` 0))))

(event `DzX_RadialMenu_Interface.RadialButtonClick`
  (params (RadialMenu :type "DzX_RadialMenu Object Reference"))
  ;[1 1 1] OnClick
  (`Widget.RemoveFromParent` RadialMenu)
  (`GameplayStatics.PlaySound2D` "/Game/StarterContent/Audio/Explosion02.Explosion02" 1.0 1.0 0.0 null null))

(event `DzX_RadialMenu_Interface.RadialMenuHoverOver`
  (params (RadialMenu :type "DzX_RadialMenu Object Reference"))
  ;[1 1 1] Hover
  (`GameplayStatics.PlaySound2D` "/Game/StarterContent/Audio/Explosion01.Explosion01" 1.0 1.0 0.0 null null))

(fn `UserConstructionScript`)