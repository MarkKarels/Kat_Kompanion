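; BP_HealthFountain is a healing fountain actor that periodically heals actors standing in its range.
; Collision overlaps maintain the in-range list, and a looping timer calls Heal on each member's BPC_EasyHealthSystem component.
; Unless Infinite, it destroys itself once CurrentTick exceeds Ticks, with the counter rising per heal rather than per timer tick.
; A RingRotation timeline spins the two rings on different axes.
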(event `self.ReceiveBeginPlay`
  ;[0.04688 0.04688 0.04688] Fountain Functionality
  ;;[0.1812 0 1] Setup
  (`KismetSystemLibrary.K2_SetTimerDelegate` (delegate `FountainTick`) (`self.Speed`) true)
  (bind (_direction _rotation) (`Timeline|RingRotation` :!via `PlayFromStart`)
    (:`Update`
      (bind _returnvalue (`KismetMathLibrary.Lerp` 0.0 360.0 _rotation))
      (`SceneComponent.K2_SetWorldRotation` (`self.Ring1`) (`KismetMathLibrary.MakeRotator` 0.0 _returnvalue) false false)
      (`SceneComponent.K2_SetWorldRotation` (`self.Ring`) (`KismetMathLibrary.MakeRotator` _returnvalue) false false))))

(event `FountainTick`
  ;[0.04688 0.04688 0.04688] Fountain Functionality
  ;;[0.1812 0 1] Functionality
  (if (`self.Infinite`)
    (for _array_element (`self.CharactersInRange`) :!label _label
      (bind _returnvalue (`self.GetComponentByClass` _array_element "/Game/EasyHealthSystem/Blueprints/BPC_EasyHealthSystem.BPC_EasyHealthSystem_C"))
      (`/Engine/EditorBlueprintResources/StandardMacros.IsValid` _returnvalue
        (:`Is Valid`
          (`/Game/EasyHealthSystem/Blueprints/BPC_EasyHealthSystem.Heal` _returnvalue (`self.HealAmount`))
          (`/Engine/EditorBlueprintResources/StandardMacros.IncrementInt` (`self.CurrentTick`)))))
    (elif (> (`self.CurrentTick`) (`self.Ticks`))
      (`self.K2_DestroyActor`)
      (else
        (goto _label)))))

(event `self.Collision.OnComponentBeginOverlap`
  (params (OverlappedComponent :type "PrimitiveComponent Object Reference") (OtherActor :type "Actor Object Reference") (OtherComp :type "PrimitiveComponent Object Reference") (OtherBodyIndex :type Integer) (bFromSweep :type Boolean) (SweepResult :type "HitResult Structure (by ref)"))
  ;[0.04688 0.04688 0.04688] Fountain Functionality
  ;;[0.1812 0 1] Enter / Leave range
  (`KismetArrayLibrary.Array_Add` (`self.CharactersInRange`) OtherActor))

(event `self.Collision.OnComponentEndOverlap`
  (params (OverlappedComponent :type "PrimitiveComponent Object Reference") (OtherActor :type "Actor Object Reference") (OtherComp :type "PrimitiveComponent Object Reference") (OtherBodyIndex :type Integer))
  ;[0.04688 0.04688 0.04688] Fountain Functionality
  ;;[0.1812 0 1] Enter / Leave range
  (`KismetArrayLibrary.Array_RemoveItem` (`self.CharactersInRange`) OtherActor))

(fn `UserConstructionScript`)