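; BP_HealthPickup3 is a health pickup that floats and spins until the Kat_2 character overlaps it.
; A Float timeline started at BeginPlay drives the Health component's height and yaw.
; Sphere overlap heals through the actor's BPC_EasyHealthSystem, guarded by a DoOnce that resets if that component is missing.
; A successful pickup plays sound and Niagara effects, animates the mesh scale with a second timeline, then destroys itself.
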(event `self.ReceiveBeginPlay`
  ;[0.01042 0.01042 0.01042] Health Pickup
  ;;[0.1812 0 1] Float Animation
  (bind (_direction _height _rotation) (`Timeline|Float` :!via `PlayFromStart`)
    (:`Update`
      (`SceneComponent.K2_SetRelativeLocation` (`self.Health`) (`KismetMathLibrary.MakeVector` 0.0 0.0 (`KismetMathLibrary.Lerp` 0.0 20.0 _height)) false false)
      (`SceneComponent.K2_SetWorldRotation` (`self.Health`) (`KismetMathLibrary.MakeRotator` 0.0 0.0 (`KismetMathLibrary.Lerp` 0.0 360.0 _rotation)) false false))))

(event `self.Sphere.OnComponentBeginOverlap`
  (params (OverlappedComponent :type "PrimitiveComponent Object Reference") (OtherActor :type "Actor Object Reference") (OtherComp :type "PrimitiveComponent Object Reference") (OtherBodyIndex :type Integer) (bFromSweep :type Boolean) (SweepResult :type "HitResult Structure (by ref)"))
  (bind _returnvalue (`self.GetComponentByClass` OtherActor "/Game/EasyHealthSystem/Blueprints/BPC_EasyHealthSystem.BPC_EasyHealthSystem_C"))
  ;[0.01042 0.01042 0.01042] Health Pickup
  ;;[0.1812 0 1] Pickup
  (cast `/Game/ThirdPerson/Blueprints/Kat_2` OtherActor)
  (`/Engine/EditorBlueprintResources/StandardMacros.DoOnce` false :!label _label
    (:`Completed`
      (`/Engine/EditorBlueprintResources/StandardMacros.IsValid` _returnvalue
        (:`Is Valid`
          (`/Game/EasyHealthSystem/Blueprints/BPC_EasyHealthSystem.Heal` _returnvalue (`self.Amount`))
          (`GameplayStatics.PlaySoundAtLocation` "/Game/EasyHealthSystem/Demo/Audio/WAV/AU_HealthPickup.AU_HealthPickup" (`SceneComponent.K2_GetComponentLocation` (`self.DefaultSceneRoot`)) (struct) 1.0 1.0 0.0 null null null null)
          (`NiagaraFunctionLibrary.SpawnSystemAtLocation` "/Game/EasyHealthSystem/Demo/Particles/NS_HealthPickup.NS_HealthPickup" (`self.K2_GetActorLocation`))
          (bind (_direction _scale) (`Timeline|DestroyAnimation` :!via `PlayFromStart`)
            (:`Update`
              (`SceneComponent.K2_SetRelativeTransform` (`self.Health`) (`KismetMathLibrary.MakeTransform` (0.0 0.0 0.0) (struct) (`KismetMathLibrary.VLerp` (0.0 0.0 0.0) (0.5 0.5 0.5) _scale)) false false))
            (:`Finished`
              (`self.K2_DestroyActor`))))
        (:`Is Not Valid`
          (goto _label :!via `Reset`))))))

(fn `UserConstructionScript`)