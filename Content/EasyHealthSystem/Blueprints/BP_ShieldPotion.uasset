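; BP_ShieldPotion is a pickup that restores shield to actors carrying a BPC_EasyHealthSystem component.
; A timeline bobs and spins the pickup mesh from BeginPlay.
; Sphere overlap calls RestoreShield with Amount, plays a sound, spawns a Niagara effect, then animates the mesh scale before destroying the actor.
; A DoOnce guards against repeat triggers and resets when the overlapping actor lacks the component.
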(event `self.ReceiveBeginPlay`
  ;[0.005208 0.005208 0.005208] Regen Pickup
  ;;[0.1812 0 1] Float Animation
  (bind (_direction _height _rotation) (`Timeline|Timeline_0` :!via `PlayFromStart`)
    (:`Update`
      (`SceneComponent.K2_SetRelativeLocation` (`self.Pickup`) (`KismetMathLibrary.MakeVector` 0.0 0.0 (`KismetMathLibrary.Lerp` 0.0 20.0 _height)) false false)
      (`SceneComponent.K2_SetWorldRotation` (`self.Pickup`) (`KismetMathLibrary.MakeRotator` 0.0 0.0 (`KismetMathLibrary.Lerp` 0.0 360.0 _rotation)) false false))))

(event `self.Sphere.OnComponentBeginOverlap`
  (params (OverlappedComponent :type "PrimitiveComponent Object Reference") (OtherActor :type "Actor Object Reference") (OtherComp :type "PrimitiveComponent Object Reference") (OtherBodyIndex :type Integer) (bFromSweep :type Boolean) (SweepResult :type "HitResult Structure (by ref)"))
  (bind _returnvalue (`self.GetComponentByClass` OtherActor "/Game/EasyHealthSystem/Blueprints/BPC_EasyHealthSystem.BPC_EasyHealthSystem_C"))
  ;[0.005208 0.005208 0.005208] Regen Pickup
  ;;[0.1812 0 1] Pickup
  (`/Engine/EditorBlueprintResources/StandardMacros.DoOnce` false :!label _label
    (:`Completed`
      (`/Engine/EditorBlueprintResources/StandardMacros.IsValid` _returnvalue
        (:`Is Valid`
          (`/Game/EasyHealthSystem/Blueprints/BPC_EasyHealthSystem.RestoreShield` _returnvalue (`self.Amount`))
          (`GameplayStatics.PlaySoundAtLocation` "/Game/EasyHealthSystem/Demo/Audio/CUE/CUE_RegenPickup.CUE_RegenPickup" (`self.K2_GetActorLocation`) (struct) 1.0 1.0 0.0 null null null null)
          (`NiagaraFunctionLibrary.SpawnSystemAtLocation` "/Game/EasyHealthSystem/Demo/Particles/NS_ShieldPotion.NS_ShieldPotion" (+ (`self.K2_GetActorLocation`) (0.0 0.0 50.0)))
          (bind (_direction _scale) (`Timeline|Timeline_1` :!via `PlayFromStart`)
            (:`Update`
              (`SceneComponent.K2_SetRelativeTransform` (`self.Pickup`) (`KismetMathLibrary.MakeTransform` (0.0 0.0 0.0) (struct) (`KismetMathLibrary.VLerp` (0.0 0.0 0.0) (0.3 0.3 0.3) _scale)) false false))
            (:`Finished`
              (`self.K2_DestroyActor`))))
        (:`Is Not Valid`
          (goto _label :!via `Reset`))))))

(fn `UserConstructionScript`)