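; Health component that gives its owning actor health, optional shield, bleeding and regeneration, destroying the owner at zero health.
; TakeDamage drains shield first, spilling the excess into health, and plays feedback sounds.
; Bleed and Regenerate apply ticks through Delay loops; a new bleed replaces an active one if stronger or the current one is about half done.
; A looping timer restores shield through a gate that damage closes and a retriggerable delay reopens.
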(event `Bleed`
  (params (Ticks :type Integer) (Speed :type "Float (double-precision)") (Damage :type "Float (double-precision)"))
  ;[0.03646 0.03646 0.03646] Health Systems
  ;;[0.1318 0 1] Bleeding
  (if (`self.IsBleeding`)
    (bind _superior (`self.CalculateSuperiorBleed` (* Ticks Damage)))
    (if _superior
      (set `self.BleedIndex` 0 :!label _label)
      (`self.UpdateBleed` Ticks Speed Damage)
      (if (> (`self.BleedIndex`) (- (`self.Ticks`) 1)) :!label _label_2
        (set `self.BleedIndex` 0)
        (set `self.IsBleeding` false)
        (else
          (`self.TakeDamage` (`self.Damage`))
          (`/Engine/EditorBlueprintResources/StandardMacros.IncrementInt` (`self.BleedIndex`)
            (:`  `
              (`NiagaraFunctionLibrary.SpawnSystemAtLocation` "/Game/EasyHealthSystem/Demo/Particles/NS_Bleed.NS_Bleed" (+ (`Actor.K2_GetActorLocation` (`self.GetOwner`)) (`KismetMathLibrary.MakeVector` 0.0 0.0 (`self.CharacterHeightCorrection`))))
              (`KismetSystemLibrary.Delay` (`self.Speed`))
              (goto _label_2)))))
      (elif (> (`KismetMathLibrary.Conv_IntToDouble` (/ (`self.BleedIndex`) (- (`self.Ticks`) 1))) 0.49)
        (goto _label)))
    (else
      (set `self.BleedIndex` 0)
      (`self.UpdateBleed` Ticks Speed Damage)
      (set `self.IsBleeding` true)
      (goto _label_2))))

(event `Regenerate`
  (params (Ticks :type Integer) (Speed :type "Float (double-precision)") (Amount :type "Float (double-precision)"))
  ;[0.03646 0.03646 0.03646] Health Systems
  ;;[0.1835 0 1] Regeneration
  (bind _output_get (set `self.RegenIndex` 0))
  (if (> _output_get (- Ticks 1)) :!label _label_3
    (set `self.RegenIndex` 0)
    (else
      (`self.Heal` Amount)
      (`/Engine/EditorBlueprintResources/StandardMacros.IncrementInt` (`self.RegenIndex`)
        (:`  `
          (`KismetSystemLibrary.Delay` Speed)
          (goto _label_3))))))

(event `self.ReceiveBeginPlay`
  (`self.Setup`)
  (`KismetSystemLibrary.K2_SetTimerDelegate` (delegate `TryRestoreShield`) (`self.ShieldRestoreSpeed`) true))

(event `TryRestoreShield`
  (`/Engine/EditorBlueprintResources/StandardMacros.Gate` true :!label _label_4
    (:`Exit`
      (`self.RestoreShield` (`self.ShieldRestoreAmount`)))))

(event `InCombatUpdate`
  (`KismetSystemLibrary.RetriggerableDelay` (`self.RestoreShieldDelay`))
  (goto _label_4 :!via `Open`))

(event `DamageTaken`
  (`self.InCombatUpdate`)
  (goto _label_4 :!via `Close`))

(fn `CalculateSuperiorBleed`
  (params (Total :type "Float (double-precision)"))
  (returns (Superior :type Boolean))
  (if (> Total (`self.OldBleedTotal`))
    (set `self.OldBleedTotal` Total)
    (return true)
    (else
      (return false))))

(fn `Death`
  (`Actor.K2_DestroyActor` (`self.GetOwner`)))

(fn `Heal`
  (params (Amount :type "Float (double-precision)"))
  (bind _output_get (set `self.Health` (+ (`self.Health`) Amount)))
  (if (> _output_get (`self.MaxHealth`))
    (set `self.Health` (`self.MaxHealth`))))

(fn `RestoreShield`
  (params (Amount :type "Float (double-precision)"))
  (if (not (== (`self.Shield`) (`self.MaxShield`)))
    (bind _output_get (set `self.Shield` (+ (`self.Shield`) Amount)))
    (`GameplayStatics.PlaySound2D` null 1.0 1.0 0.0 null null)
    (if (> _output_get (`self.MaxShield`))
      (set `self.Shield` (`self.MaxShield`)))))

(fn `Setup`
  (set `self.Shield` (`self.MaxShield`))
  (set `self.Health` (`self.MaxHealth`)))

(fn `TakeDamage`
  (params (Damage :type "Float (double-precision)"))
  (locals (DamageAmount :type "Float (double-precision)") (CurrentShieldAmount :type "Float (double-precision)"))
  (bind _returnvalue (- (`self.Shield`) (`local.DamageAmount`)))
  (`GameplayStatics.PlaySound2D` (`self.DamageSound`) 1.0 1.0 0.0 null null)
  (`self.DamageTaken`)
  (set `local.DamageAmount` Damage)
  (if (`self.CharacterHasShield`)
    (if (> (`self.Shield`) 0.0)
      (if (> _returnvalue 0.0)
        (set `self.Shield` _returnvalue)
        (else
          (bind _output_get (set `self.Health` (- (`self.Health`) (- (`local.DamageAmount`) (`self.Shield`)))))
          (set `self.Shield` 0.0)
          (`GameplayStatics.PlaySound2D` (`self.ShieldDestroyedSound`) 1.0 1.0 0.0 null null)
          (if (<= _output_get 0.0)
            (`GameplayStatics.PlaySound2D` (`self.DeathSound`) 1.0 1.0 0.0 null null)
            (`self.Death`))))
      (else
        (bind _output_get_2 (set `self.Health` (- (`self.Health`) (`local.DamageAmount`)) :!label _label))
        (if (<= _output_get_2 0.0)
          (`GameplayStatics.PlaySound2D` (`self.DeathSound`) 1.0 1.0 0.0 null null)
          (`self.Death`))))
    (else
      (goto _label))))

(fn `UpdateBleed`
  (params (Ticks :type Integer) (Speed :type "Float (double-precision)") (Damage :type "Float (double-precision)"))
  (bind _output_get (set `self.Ticks` Ticks))
  (set `self.Speed` Speed)
  (set `self.Damage` Damage)
  (set `self.OldBleedTotal` (* _output_get Damage)))