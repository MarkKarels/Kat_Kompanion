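; Konrad is a dialogue NPC that can follow the player and play a greeting with animation, sound and printed prompt.
; On BeginPlay it spawns a dialogue actor, filled from DataTables when one is valid, otherwise using default entries.
; Sphere overlaps toggle a talk widget, shown only while not following.
; Following re-issues AI MoveTo on a short delay loop; construction attaches clothes and backpack meshes via master pose.
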(event `self.ReceiveBeginPlay`
  ;[0.2135 0.2135 0.2135] Event Begin Play
  (`self.Spawn Dialogue Actor`)
  (bind _asprotagonist (cast `/Game/ThirdPerson/Blueprints/Protagonist` (`GameplayStatics.GetPlayerCharacter` 0)))
  (set `self.Char REF` _asprotagonist))

(event `self.Sphere.OnComponentBeginOverlap`
  (params (OverlappedComponent :type "PrimitiveComponent Object Reference") (OtherActor :type "Actor Object Reference") (OtherComp :type "PrimitiveComponent Object Reference") (OtherBodyIndex :type Integer) (bFromSweep :type Boolean) (SweepResult :type "HitResult Structure (by ref)"))
  ;[0.2135 0.2135 0.2135] Show and hide speech widget above character
  (if (not (`self.FollowPlayer?`))
    (`self.Toggle Talk Notification Widget` OtherActor true)))

(event `self.Sphere.OnComponentEndOverlap`
  (params (OverlappedComponent :type "PrimitiveComponent Object Reference") (OtherActor :type "Actor Object Reference") (OtherComp :type "PrimitiveComponent Object Reference") (OtherBodyIndex :type Integer))
  ;[0.2135 0.2135 0.2135] Show and hide speech widget above character
  (`self.Toggle Talk Notification Widget` OtherActor))

(event `Follow Player`
  ;[1 1 1] AI Follow
  (if (`self.FollowPlayer?`)
    (if (>= (`self.GetDistanceTo` (`self.Char REF`)) 200.0)
      (`|AIMoveTo` self (0.0 0.0 0.0) (`self.Char REF`) 10.0
        (:`then`
          _))
      (else
        (`|AIMoveTo` self (0.0 0.0 0.0) (`self.Char REF`) 10.0 :!label _label
          (:`then`
            _))))
    (`KismetSystemLibrary.Delay` 0.1)
    (`self.Follow Player`)))

(event `Stop Movement`
  ;[1 1 1] AI Follow
  (goto _label))

(event `Hello Dance`
  ;[1 1 1] Greeting
  (`GameplayStatics.PlaySound2D` "/Game/Audio/hello-87032.hello-87032" 1.0 1.0 0.0 null null)
  (`SkeletalMeshComponent.PlayAnimation` (`self.Mesh`) "/Game/Kitty/Animations/Anim_Attack2_Retargeted.Anim_Attack2_Retargeted" false)
  (`KismetSystemLibrary.Delay` 1.8)
  (`SkeletalMeshComponent.SetAnimationMode` (`self.Mesh`) "AnimationBlueprint")
  (`GameplayStatics.PlaySound2D` "/Game/Audio/KristophIntro.KristophIntro" 1.0 1.0 0.0 null null)
  (`KismetSystemLibrary.PrintString` "Hey Friend! come over here and press the E key, or the A button on your game pad so I can tell you something."))

(fn `Spawn Dialogue Actor`
  (if (`self.Contains Dialogue`)
    (`/Engine/EditorBlueprintResources/StandardMacros.IsValid` (`self.Dialogue Data Table`)
      (:`Is Valid`
        ;[0.2135 0.2135 0.2135] Initialize data table
        (bind _dialogue_data_table (`self.Dialogue Data Table`)
          (:`then`
            (bind _outrownames (`DataTableFunctionLibrary.GetDataTableRowNames` _dialogue_data_table))
            (for _array_element _outrownames
              (bind _returnvalue (`|GetDataTableRow` _dialogue_data_table _array_element)
                (:`then`
                  (`KismetArrayLibrary.Array_Add` (`self.Dialogue Entries`) _returnvalue)))))
          (:`else`
            _))
        (bind _choice_01_data_table (`self.Choice 01 Data Table`)
          (:`then`
            (bind _outrownames_2 (`DataTableFunctionLibrary.GetDataTableRowNames` _choice_01_data_table))
            (for _array_element_2 _outrownames_2
              (bind _returnvalue_2 (`|GetDataTableRow` _choice_01_data_table _array_element_2)
                (:`then`
                  (`KismetArrayLibrary.Array_Add` (`self.Choice 01 Response`) _returnvalue_2)))))
          (:`else`
            _))
        (bind _choice_02_data_table (`self.Choice 02 Data Table`)
          (:`then`
            (bind _outrownames_3 (`DataTableFunctionLibrary.GetDataTableRowNames` _choice_02_data_table))
            (for _array_element_3 _outrownames_3
              (bind _returnvalue_3 (`|GetDataTableRow` _choice_02_data_table _array_element_3)
                (:`then`
                  (`KismetArrayLibrary.Array_Add` (`self.Choice 02 Response`) _returnvalue_3)))))
          (:`else`
            _))
        (`|SpawnActorFromClass` "/Game/EasyRPGDialogueSystem/Blueprints/Actors/BP_DialogueDataTables.BP_DialogueDataTables_C" (`self.GetTransform`) "Undefined" "OverrideRootScale" null (`self.Dialogue Entries`) (`self.Contains Choice`) (`self.Choices Loop`) (`self.Choice 01`) (`self.Choice 02`) (`self.Choice 01 Response`) (`self.Choice 02 Response`) (`self.NPC Rotates`) self null))
      (:`Is Not Valid`
        ;[0.2135 0.2135 0.2135] Initialize Default
        (`|SpawnActorFromClass` "/Game/EasyRPGDialogueSystem/Blueprints/Actors/BP_Dialogue.BP_Dialogue_C" (`self.GetTransform`) "Undefined" "OverrideRootScale" null (`self.Dialogue Entries`) (`self.Contains Choice`) (`self.Choices Loop`) (`self.Choice 01`) (`self.Choice 02`) (`self.Choice 01 Response`) (`self.Choice 02 Response`) (`self.NPC Rotates`) self null)))))

(fn `Toggle Talk Notification Widget`
  (params (Target :type "Actor Object Reference") (bNewVisibility :type Boolean))
  (if (`self.Contains Dialogue`)
    (cast `/Game/ThirdPerson/Blueprints/Protagonist` (`self.GetInstigator` Target))
    (`SceneComponent.SetVisibility` (`self.Talk Widget`) bNewVisibility false)))

(fn `UserConstructionScript`
  (bind _clothes (`self.Clothes`))
  (bind _backpack (`self.Backpack`))
  (`|ExecutionSequence`
    (:`then_0`
      (`SkinnedMeshComponent.SetSkinnedAssetAndUpdate` _clothes "/Game/Kitty/Mesh/SK_Kitty_Clothes.SK_Kitty_Clothes" true)
      (`SkinnedMeshComponent.SetLeaderPoseComponent` _clothes (`self.Mesh`) false))
    (:`then_1`
      (`SkinnedMeshComponent.SetSkinnedAssetAndUpdate` _backpack "/Game/Kitty/Mesh/SK_Kitty_BackPack.SK_Kitty_BackPack" true)
      (`SkinnedMeshComponent.SetLeaderPoseComponent` _backpack (`self.Mesh`) false))))